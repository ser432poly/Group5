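; BP_SisterNPC is the sister NPC, which shows dialog widgets when its box is overlapped.
; Begin overlap reads the State of the first BP_BrotherNPC, showing SisterDialogPresent1 at zero, or otherwise SisterDialogPresent2 if that brother's first overlapping EarthPrince is the player.
; End overlap repeats the check to remove the matching widget.
; The construction script tints the pawn mesh blue through a dynamic material.
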(event OnComponentBeginOverlap(Box)
  (params (OtherActor :type Actor%20Object%20Reference) (OtherComp :type Primitive%20Component%20Object%20Reference) (OtherBodyIndex :type Integer) (bFromSweep :type Boolean) (SweepResult :type Hit%20Result%20Structure%20%28by%20ref%29))
  (bind _outactors (Actor|GetAllActorsOfClass "/Game/Blueprints/Pawns/BP_BrotherNPC.BP_BrotherNPC_C"))
  (if (== (Variables|/Game/Blueprints/Pawns/BP_BrotherNPC.BP_BrotherNPC_C|Getstate (Utilities|Array|Get(acopy) _outactors)) 0)
    (bind _returnvalue (UserInterface|CreateWidget "/Game/Blueprints/Actors/NPC/Geography/SisterDialogPresent1.SisterDialogPresent1_C"))
    (UserInterface|Viewport|AddtoViewport _returnvalue 0)
    (elif (== (Utilities|Array|Get(acopy) (Collision|GetOverlappingActors (Utilities|Array|Get(acopy) _outactors) "/Game/Blueprints/Pawns/EarthPrince.EarthPrince_C" :!class /Script/Engine.Actor)) (Game|GetPlayerCharacter 0))
      (bind _returnvalue_2 (UserInterface|CreateWidget "/Game/Blueprints/Actors/NPC/Geography/SisterDialogPresent2.SisterDialogPresent2_C"))
      (UserInterface|Viewport|AddtoViewport _returnvalue_2 0))))

(event OnComponentEndOverlap(Box)
  (params (OtherActor :type Actor%20Object%20Reference) (OtherComp :type Primitive%20Component%20Object%20Reference) (OtherBodyIndex :type Integer))
  (bind _outactors (Actor|GetAllActorsOfClass "/Game/Blueprints/Pawns/BP_BrotherNPC.BP_BrotherNPC_C"))
  (if (== (Variables|/Game/Blueprints/Pawns/BP_BrotherNPC.BP_BrotherNPC_C|Getstate (Utilities|Array|Get(acopy) _outactors)) 0)
    (Widget|RemovefromParent (stale OnComponentBeginOverlap(Box) _returnvalue))
    (elif (== (Utilities|Array|Get(acopy) (Collision|GetOverlappingActors (Utilities|Array|Get(acopy) (stale OnComponentBeginOverlap(Box) _outactors)) "/Game/Blueprints/Pawns/EarthPrince.EarthPrince_C" :!class /Script/Engine.Actor)) (Game|GetPlayerCharacter 0))
      (Widget|RemovefromParent (stale OnComponentBeginOverlap(Box) _returnvalue_2)))))

(fn ConstructionScript
  (bind _pawnmesh (Variables|Default|GetPawnMesh))
  (bind _returnvalue (Rendering|Material|CreateDynamicMaterialInstance _pawnmesh 0 (Utilities|Array|Get(acopy) (Rendering|Material|GetMaterials _pawnmesh)) :!class /Script/Engine.PrimitiveComponent))
  (Rendering|Material|SetVectorParameterValue _returnvalue "BodyColor" "(R=0.057249,G=0.000000,B=1.000000,A=0.000000)" :!class /Script/Engine.MaterialInstanceDynamic))