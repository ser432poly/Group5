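; BP_Businessman is a quest-giver NPC that sets a star-collection goal and judges the player's count.
; The first box overlap opens an intro dialog, whose end event starts the game with a random goal and broadcasts both.
; Later overlaps show a correct or incorrect dialog on an exact star match, with the correct one triggering a level-complete dispatcher.
; Leaving removes dialogs; the construction script tints the body red.
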(event OnComponentBeginOverlap(Box)
  (params (OtherActor :type Actor%20Object%20Reference) (OtherComp :type Primitive%20Component%20Object%20Reference) (OtherBodyIndex :type Integer) (bFromSweep :type Boolean) (SweepResult :type Hit%20Result%20Structure%20%28by%20ref%29))
  (bind _asbp_third_person_character (Utilities|Casting|CastToBP_ThirdPersonCharacter OtherActor))
  (if (Variables|Default|GetGameStart)
    (if (== (Variables|Default|GetGoal) (Variables|/Game/Blueprints/Pawns/BP_ThirdPersonCharacter.BP_ThirdPersonCharacter_C|GetStar _asbp_third_person_character))
      (bind _returnvalue (UserInterface|CreateWidget "/Game/Blueprints/Actors/NPC/Businessman/BusinessmanCorrectDialogPresent.BusinessmanCorrectDialogPresent_C"))
      (UserInterface|Viewport|AddtoViewport _returnvalue 0)
      (EventDispatchers|AssignLevelComplete _returnvalue (delegate Custom|LevelComplete_Event_0))
      (else
        ;[1 1 1] Player Collect Incorrect Number of Stars
        (bind _returnvalue_2 (UserInterface|CreateWidget "/Game/Blueprints/Actors/NPC/Businessman/BusinessmanIncorrectDialogPresent.BusinessmanIncorrectDialogPresent_C"))
        (UserInterface|Viewport|AddtoViewport _returnvalue_2 0)))
    (else
      ;[1 1 1] Trigger Initial Conversation
      (bind _returnvalue_3 (UserInterface|CreateWidget "/Game/Blueprints/Actors/NPC/Businessman/BusinessmanDialogPresent.BusinessmanDialogPresent_C"))
      (UserInterface|Viewport|AddtoViewport _returnvalue_3 0)
      (EventDispatchers|AssignEndBusinessmanInital _returnvalue_3 (delegate Custom|EndBusinessmanInital_Event_0)))))

(event OnComponentEndOverlap(Box)
  (params (OtherActor :type Actor%20Object%20Reference) (OtherComp :type Primitive%20Component%20Object%20Reference) (OtherBodyIndex :type Integer))
  ;[1 1 1] Trigger Initial Conversation
  (Utilities|Casting|CastToBP_ThirdPersonCharacter OtherActor)
  (Widget|RemovefromParent (stale OnComponentBeginOverlap(Box) _returnvalue_3)))

(event Custom|EndBusinessmanInital_Event_0
  (params (ConvoEnd :type Boolean))
  ;[1 1 1] Trigger Initial Conversation
  (bind _output_get (Variables|Default|SetGameStart ConvoEnd))
  (bind _output_get_2 (Variables|Default|SetGoal (Math|Random|RandomIntegerinRange 100 500)))
  (Default|CallSetGameStart _output_get _output_get_2))

(event Custom|LevelComplete_Event_0
  (Default|CallSetLevelComplete))

(fn ConstructionScript
  (bind _pawnmesh (Variables|Default|GetPawnMesh))
  (bind _returnvalue (Rendering|Material|CreateDynamicMaterialInstance _pawnmesh 0 (Utilities|Array|Get(acopy) (Rendering|Material|GetMaterials _pawnmesh)) :!class /Script/Engine.PrimitiveComponent))
  (Rendering|Material|SetVectorParameterValue _returnvalue "BodyColor" "(R=1.000000,G=0.000000,B=0.000000,A=0.000000)" :!class /Script/Engine.MaterialInstanceDynamic))