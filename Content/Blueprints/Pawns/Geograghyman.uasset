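; Geographyman pawn that shows dialog widgets when something overlaps its Box, acting as a geography-themed character.
; State 0 shows the geography dialog and state 2 the end dialog; leaving the Box removes the widget matching the current state.
; SetFinalStategamewin switches State to 2, the game-win stage.
; The construction script tints the pawn mesh red through a dynamic material instance.
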(event OnComponentBeginOverlap(Box)
  (params (OtherActor :type Actor%20Object%20Reference) (OtherComp :type Primitive%20Component%20Object%20Reference) (OtherBodyIndex :type Integer) (bFromSweep :type Boolean) (SweepResult :type Hit%20Result%20Structure%20%28by%20ref%29))
  (if (== (Variables|Default|Getstate) 0)
    (bind _returnvalue (UserInterface|CreateWidget "/Game/Blueprints/Actors/NPC/Geography/GeographyDialogPresent.GeographyDialogPresent_C"))
    (UserInterface|Viewport|AddtoViewport _returnvalue 0)
    (elif (== (Variables|Default|Getstate) 2)
      (bind _returnvalue_2 (UserInterface|CreateWidget "/Game/Blueprints/Actors/NPC/Geography/EndDialogPresent.EndDialogPresent_C"))
      (UserInterface|Viewport|AddtoViewport _returnvalue_2 0))))

(event OnComponentEndOverlap(Box)
  (params (OtherActor :type Actor%20Object%20Reference) (OtherComp :type Primitive%20Component%20Object%20Reference) (OtherBodyIndex :type Integer))
  (if (== (Variables|Default|Getstate) 0)
    (Widget|RemovefromParent (stale OnComponentBeginOverlap(Box) _returnvalue))
    (elif (== (Variables|Default|Getstate) 2)
      (Widget|RemovefromParent (stale OnComponentBeginOverlap(Box) _returnvalue_2)))))

(fn ConstructionScript
  (bind _pawnmesh (Variables|Default|GetPawnMesh))
  (bind _returnvalue (Rendering|Material|CreateDynamicMaterialInstance _pawnmesh 0 (Utilities|Array|Get(acopy) (Rendering|Material|GetMaterials _pawnmesh)) :!class /Script/Engine.PrimitiveComponent))
  (Rendering|Material|SetVectorParameterValue _returnvalue "BodyColor" "(R=1.000000,G=0.000000,B=0.000000,A=0.000000)" :!class /Script/Engine.MaterialInstanceDynamic))

(fn SetFinalStategamewin
  (Variables|Default|Setstate 2))