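; BP_BrotherNPC is the brother NPC pawn, which shows a dialog prompt and can follow the player.
; In State 0, overlapping its Box adds a BrotherDialogPresent widget, and ending the overlap removes it, with no active check on the overlapping actor.
; In State 1, Tick reissues AIMoveTo toward the player every frame; State is not changed here.
; The construction script tints the body green through a dynamic material instance.
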(event OnComponentBeginOverlap(Box)
  (params (OtherActor :type Actor%20Object%20Reference) (OtherComp :type Primitive%20Component%20Object%20Reference) (OtherBodyIndex :type Integer) (bFromSweep :type Boolean) (SweepResult :type Hit%20Result%20Structure%20%28by%20ref%29))
  (if (== (Variables|Default|Getstate) 0)
    (bind _returnvalue (UserInterface|CreateWidget "/Game/Blueprints/Actors/NPC/Geography/BrotherDialogPresent.BrotherDialogPresent_C"))
    (UserInterface|Viewport|AddtoViewport _returnvalue 0)))

(event OnComponentEndOverlap(Box)
  (params (OtherActor :type Actor%20Object%20Reference) (OtherComp :type Primitive%20Component%20Object%20Reference) (OtherBodyIndex :type Integer))
  (Widget|RemovefromParent (stale OnComponentBeginOverlap(Box) _returnvalue)))

(event EventTick
  (params (DeltaSeconds :type Float%20%28single-precision%29))
  (if (== (Variables|Default|Getstate) 1)
    (AI|AIMoveTo self "0, 0, 0" (Game|GetPlayerCharacter 0) 1e+01 false)))

(fn ConstructionScript
  (bind _pawnmesh (Variables|Default|GetPawnMesh))
  (bind _returnvalue (Rendering|Material|CreateDynamicMaterialInstance _pawnmesh 0 (Utilities|Array|Get(acopy) (Rendering|Material|GetMaterials _pawnmesh)) :!class /Script/Engine.PrimitiveComponent))
  (Rendering|Material|SetVectorParameterValue _returnvalue "BodyColor" "(R=0.000000,G=1.000000,B=0.002356,A=0.000000)" :!class /Script/Engine.MaterialInstanceDynamic))