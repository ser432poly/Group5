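; BP_Crystal is a short-lived crystal pickup that the EarthPrince collects by overlapping it.
; On BeginPlay a chain of delays swaps the cube's material twice as a countdown cue, then destroys the actor after about eight seconds.
; On overlap it casts to EarthPrince, increments that actor's CrystalCollected count, prints the total and destroys itself.
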(event EventBeginPlay
  ;[1 1 1] Spawn crystals for 8 seconds total
  ;;[1 1 1] as timer drops, change colour.
  (Utilities|FlowControl|Delay 3.5)
  (Rendering|Material|SetMaterial (Variables|Default|GetCube) 0 "/Game/WaterPlane/Lake/Materials/M_LakeWater_02.M_LakeWater_02")
  (Utilities|FlowControl|Delay 2.0)
  (Rendering|Material|SetMaterial (Variables|Default|GetCube) 0 "/Game/WaterPlane/Lake/Materials/M_LakeWater_03.M_LakeWater_03")
  (Utilities|FlowControl|Delay 2.0)
  (Actor|DestroyActor self))

(event EventActorBeginOverlap
  (params (OtherActor :type Actor%20Object%20Reference))
  (bind _asearth_prince (Utilities|Casting|CastToEarthPrince OtherActor))
  (Variables|/Game/Blueprints/Pawns/EarthPrince.EarthPrince_C|SetCrystal%20Collected _asearth_prince (+ (Variables|/Game/Blueprints/Pawns/EarthPrince.EarthPrince_C|GetCrystal%20Collected _asearth_prince) 1))
  (Development|PrintString (Utilities|String|Append (Variables|Default|GetYou%20have%20Collected) (Utilities|String|ToString(Integer) (Variables|/Game/Blueprints/Pawns/EarthPrince.EarthPrince_C|GetCrystal%20Collected _asearth_prince))))
  (Actor|DestroyActor self))

(event EventTick
  (params (DeltaSeconds :type Float%20%28single-precision%29)))

(fn ConstructionScript)