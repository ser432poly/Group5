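; BP_Star is a star actor with a Worth value and a gravity component tied to the level's asteroids.
; On BeginPlay it finds every BP_Asteroid and passes each in turn to the GravityComponent's SetCurrentPlanet.
; The construction script writes Worth as text to two components, Worth1 and Worth2.
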(event EventActorBeginOverlap
  (params (OtherActor :type Actor%20Object%20Reference)))

(event EventTick
  (params (DeltaSeconds :type Float%20%28single-precision%29)))

(event EventBeginPlay
  (bind _outactors (Actor|GetAllActorsOfClass "/Game/Blueprints/Actors/BP_Asteroid.BP_Asteroid_C"))
  (for _array_element _outactors
    (Class|CustomGravityComponent|SetCurrentPlanet (Variables|Default|GetGravityComponent) _array_element)))

(fn ConstructionScript
  (bind _worth (Variables|Default|GetWorth))
  (bind _returnvalue (Utilities|Text|ToText(Integer) _worth))
  (Rendering|Components|TextRender|SetText (Variables|Default|GetWorth_1) _returnvalue)
  (Rendering|Components|TextRender|SetText (Variables|Default|GetWorth_2) _returnvalue))