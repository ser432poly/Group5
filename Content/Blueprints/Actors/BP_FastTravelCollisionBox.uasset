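; BP_FastTravelCollisionBox is a trigger actor, named for fast travel, that so far only prints debug strings when the EarthPrince enters or leaves its Box.
; On begin overlap it prints a greeting, then gathers every Geograghyman actor in the level and prints one of two messages for each, depending on whether its State equals 2.
; End overlap only repeats the greeting, and no travel logic exists yet.
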(event OnComponentBeginOverlap(Box)
  (params (OtherActor :type Actor%20Object%20Reference) (OtherComp :type Primitive%20Component%20Object%20Reference) (OtherBodyIndex :type Integer) (bFromSweep :type Boolean) (SweepResult :type Hit%20Result%20Structure%20%28by%20ref%29))
  (Utilities|Casting|CastToEarthPrince OtherActor)
  (Development|PrintString "Hello")
  (bind _outactors (Actor|GetAllActorsOfClass "/Game/Blueprints/Pawns/Geograghyman.Geograghyman_C"))
  (for _array_element _outactors
    (bind _output_get (Variables|Default|SetGeographyman _array_element))
    (if (== (Variables|/Game/Blueprints/Pawns/Geograghyman.Geograghyman_C|Getstate _output_get) 2)
      (Development|PrintString "howdy do")
      (else
        (Development|PrintString "try again")))))

(event OnComponentEndOverlap(Box)
  (params (OtherActor :type Actor%20Object%20Reference) (OtherComp :type Primitive%20Component%20Object%20Reference) (OtherBodyIndex :type Integer))
  (Utilities|Casting|CastToEarthPrince OtherActor)
  (Development|PrintString "Hello"))

(fn ConstructionScript)