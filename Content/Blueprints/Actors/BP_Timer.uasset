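; BP_Timer is a timer actor that stops the player once a set duration has elapsed.
; BeginPlay waits SetTimer seconds, then sets the MovementComponent MaxSpeed of the player's CustomPawn to zero.
; Separately, Tick uses a one-second Delay to increment TimerCount and print it, printing "time is up" only when the count exactly equals SetTimer.
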(event EventTick
  (params (DeltaSeconds :type Float%20%28single-precision%29))
  (Utilities|FlowControl|Delay 1.0)
  (Variables|Default|Settimer%20count (+ (Variables|Default|Gettimer%20count) 1.0))
  (if (== (Variables|Default|Gettimer%20count) (Variables|Default|GetSet%20Timer))
    (Development|PrintString "time is up")
    (else
      (Development|PrintString (Utilities|String|ToString(Float) (Variables|Default|Gettimer%20count))))))

(event EventBeginPlay
  ;[1 1 1] stop player when time is up
  (bind _ascustom_pawn (Utilities|Casting|CastToCustomPawn (Game|Player|GetPlayerPawn 0)))
  (Utilities|FlowControl|Delay (Variables|Default|GetSet%20Timer))
  (Variables|/Script/Engine.FloatingPawnMovement|SetMaxSpeed (Variables|/Script/CustomGravityPlugin.CustomPawn|GetMovementComponent _ascustom_pawn) 0.0))

(fn ConstructionScript)