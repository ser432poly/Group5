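; BP_CrystalSpawner is an actor that spawns BP_Crystal pickups at random points inside its Box bounds.
; Any actor overlap turns spawning on, and a Delay in Tick paces spawns to roughly one per half second.
; When the EarthPrince player's CrystalCollected equals 50, it stops spawning, bumps the count so the branch passes once, and prints a notice.
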(event EventActorBeginOverlap
  (params (OtherActor :type Actor%20Object%20Reference))
  (Variables|Default|SetSpawning true))

(event EventTick
  (params (DeltaSeconds :type Float%20%28single-precision%29))
  (bind _box (Variables|Default|GetBox))
  (bind (_origin _boxextent) (Collision|GetComponentBounds _box))
  (bind _asearth_prince (Utilities|Casting|CastToEarthPrince (Game|Player|GetPlayerPawn 0)))
  (if (== (Variables|/Game/Blueprints/Pawns/EarthPrince.EarthPrince_C|GetCrystal%20Collected _asearth_prince) 50)
    (Variables|Default|SetSpawning false)
    (Variables|/Game/Blueprints/Pawns/EarthPrince.EarthPrince_C|SetCrystal%20Collected _asearth_prince (+ (Variables|/Game/Blueprints/Pawns/EarthPrince.EarthPrince_C|GetCrystal%20Collected _asearth_prince) 1))
    (Development|PrintString "You have enough crystal now")
    (else
      (Utilities|FlowControl|Delay 0.5)
      (if (Variables|Default|GetSpawning)
        (Game|SpawnActorfromClass "/Game/Blueprints/Actors/BP_Crystal.BP_Crystal_C" (Math|Conversions|ToTransform(Vector) (Math|Random|RandomPointinBoundingBox _origin _boxextent)) "AdjustIfPossibleButDontSpawnIfColliding" 0 0)))))

(fn ConstructionScript)