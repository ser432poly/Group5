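; BP_Mushroom is a hazard actor that costs the third-person character a random amount of Star when overlapped.
; On overlap, it casts to BP_ThirdPersonCharacter, subtracts a random integer below 30 or sets Star to zero, then prints the result.
; The branch test and the subtraction roll separately, so Star can still end up negative.
; The mushroom stays in the level afterward.
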(event Collision|EventActorBeginOverlap
  (params (OtherActor :type Actor%20Object%20Reference))
  (bind _asbp_third_person_character (Utilities|Casting|CastToBP_ThirdPersonCharacter OtherActor))
  (if (> (- (Variables|/Game/Blueprints/Pawns/BP_ThirdPersonCharacter.BP_ThirdPersonCharacter_C|GetStar _asbp_third_person_character) (Math|Random|RandomInteger 30)) 0)
    (bind _output_get (Variables|/Game/Blueprints/Pawns/BP_ThirdPersonCharacter.BP_ThirdPersonCharacter_C|SetStar _asbp_third_person_character (- (Variables|/Game/Blueprints/Pawns/BP_ThirdPersonCharacter.BP_ThirdPersonCharacter_C|GetStar _asbp_third_person_character) (Math|Random|RandomInteger 30))))
    (Development|PrintString (Utilities|String|ToString(Integer) _output_get))
    (else
      (bind _output_get_2 (Variables|/Game/Blueprints/Pawns/BP_ThirdPersonCharacter.BP_ThirdPersonCharacter_C|SetStar _asbp_third_person_character 0))
      (Development|PrintString (Utilities|String|ToString(Integer) _output_get_2)))))

(fn ConstructionScript)