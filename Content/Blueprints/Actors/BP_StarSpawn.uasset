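; BP_StarSpawn is a spawner actor that continually scatters BP_Star pickups or objects around its SphereVolume component.
; A Delay on Tick throttles spawning to roughly one star every half second.
; Each star gets a random rotation, uniform scale and position within the sphere's bounding cube, since axes are randomized independently.
; The random scale also sets the star's Worth, so larger stars are worth more.
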(event EventTick
  (params (DeltaSeconds :type Float%20%28single-precision%29))
  (bind _spherevolume (Variables|Default|GetSphereVolume))
  (bind _returnvalue (Transformation|GetWorldLocation _spherevolume))
  (bind _returnvalue_2 (Components|Sphere|GetScaledSphereRadius _spherevolume))
  (bind (_x _y _z) (Math|Vector|BreakVector _returnvalue))
  (Utilities|FlowControl|Delay 0.5)
  (Variables|Default|SetrandVal (Math|Random|RandomFloatinRange 3.0 7.0))
  (Game|SpawnActorfromClass "/Game/Blueprints/Actors/BP_Star.BP_Star_C" (Math|Transform|MakeTransform (Math|Vector|MakeVector (Math|Random|RandomFloatinRange (- _x _returnvalue_2) (+ _x _returnvalue_2)) (Math|Random|RandomFloatinRange (- _y _returnvalue_2) (+ _y _returnvalue_2)) (Math|Random|RandomFloatinRange (- _z _returnvalue_2) (+ _z _returnvalue_2))) (Math|Random|RandomRotator true) (Math|Vector|MakeVector (Variables|Default|GetrandVal) (Variables|Default|GetrandVal) (Variables|Default|GetrandVal))) "Undefined" 0 (Math|Float|Round (- 2e+01 (* (- 7.0 (Variables|Default|GetrandVal)) 5.0))) 0))

(fn ConstructionScript)